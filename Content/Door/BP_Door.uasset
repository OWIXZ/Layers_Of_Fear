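; BP_Door is a door that swings while held and shows proximity icons.
; The OpenDoor event adds relative yaw to the door mesh from the passed X value scaled by Smothness, only while IsHoldingDoor is true.
; An outer collider shows the outer icon for the player, and an inner collider swaps it for the inner icon.
; Inner overlaps respond to any actor, as their player checks are disconnected.
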(event OnComponentBeginOverlap(InnerBoxCollider)
  (params (OverlappedComponent :type Primitive%20Component%20Object%20Reference) (OtherActor :type Actor%20Object%20Reference) (OtherComp :type Primitive%20Component%20Object%20Reference) (OtherBodyIndex :type Integer) (bFromSweep :type Boolean) (SweepResult :type Hit%20Result%20Structure%20%28by%20ref%29))
  (Rendering|SetVisibility (Variables|Default|GetinnerIcon) true false)
  (Rendering|SetVisibility (Variables|Default|GetouterIcon) false false))

(event OnComponentEndOverlap(InnerBoxCollider)
  (params (OverlappedComponent :type Primitive%20Component%20Object%20Reference) (OtherActor :type Actor%20Object%20Reference) (OtherComp :type Primitive%20Component%20Object%20Reference) (OtherBodyIndex :type Integer))
  (Rendering|SetVisibility (Variables|Default|GetinnerIcon) false false)
  (Rendering|SetVisibility (Variables|Default|GetouterIcon) true false))

(event OnComponentBeginOverlap(OuterBoxCollider)
  (params (OverlappedComponent :type Primitive%20Component%20Object%20Reference) (OtherActor :type Actor%20Object%20Reference) (OtherComp :type Primitive%20Component%20Object%20Reference) (OtherBodyIndex :type Integer) (bFromSweep :type Boolean) (SweepResult :type Hit%20Result%20Structure%20%28by%20ref%29))
  (if (== OtherActor (Game|GetPlayerCharacter 0))
    (Rendering|SetVisibility (Variables|Default|GetouterIcon) true false)))

(event OnComponentEndOverlap(OuterBoxCollider)
  (params (OverlappedComponent :type Primitive%20Component%20Object%20Reference) (OtherActor :type Actor%20Object%20Reference) (OtherComp :type Primitive%20Component%20Object%20Reference) (OtherBodyIndex :type Integer))
  (if (== (Game|GetPlayerCharacter 0) OtherActor)
    (Rendering|SetVisibility (Variables|Default|GetouterIcon) false false)))

(event EventOpenDoor
  (params (X%20Value :type Float%20%28double-precision%29) (IsHoldingDoor :type Boolean) (IsLookAtDoor :type Boolean))
  (if IsHoldingDoor
    (bind _output_get (Variables|Default|SetX%20Value X%20Value))
    (Transformation|AddRelativeRotation (Variables|Default|GetDoor) (Math|Rotator|MakeRotator 0.0 0.0 (* _output_get (Variables|Default|GetSmothness))) false false)))

(fn ConstructionScript)